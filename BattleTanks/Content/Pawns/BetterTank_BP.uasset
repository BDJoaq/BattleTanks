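; Player-controllable tank pawn that wires input to C++-style movement, aiming and camera components.
; On BeginPlay it hands the tracks to TankMovement, the barrel and turret to TankAiming, and itself to the HealthBar widget.
; Axis inputs drive movement intents and rotate the gimbal and spring arm for aiming; actions fire or toggle between two cameras.
; The construction script assigns track meshes, physical material and hit notifications.
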(event EventBeginPlay
  (Class|TankMovementComponent|Initialize (Variables|Default|GetTankMovement) (Variables|Default|GetTrackLeft) (Variables|Default|GetTrackRight))
  (Class|TankAimingComponent|Initialize (Variables|Default|GetTankAiming) (Variables|Default|GetBarrel) (Variables|Default|GetTankTurret))
  (CallFunction|InitializeHealthBarWidget))

(event Input|ActionEvents|InputActionFire
  (params (Key :type Key%20Structure :default "None"))
  ;[1 1 1] Aim and fire input
  (:Pressed
    (Class|TankAimingComponent|Fire (Variables|Default|GetTankAiming))))

(event Input|ActionEvents|InputActionSwitchCam
  (params (Key :type Key%20Structure :default "None"))
  ;[1 1 1] Change Camera
  (:Pressed
    (Components|Activation|ToggleActive (Variables|Default|GetCamera))
    (Components|Activation|ToggleActive (Variables|Default|GetFPCamera))))

(event Input|AxisEvents|InputAxisAimAzimuth
  (params (AxisValue :type Float%20%28single-precision%29))
  ;[1 1 1] Aim and fire input
  (Transformation|AddLocalRotation (Variables|Default|GetAzimuthGimbal) (Math|Rotator|MakeRotator 0.0 0.0 (* AxisValue 1.5)) false false))

(event Input|AxisEvents|InputAxisAimElevation
  (params (AxisValue :type Float%20%28single-precision%29))
  ;[1 1 1] Aim and fire input
  (Transformation|AddLocalRotation (Variables|Default|GetSpringArm) (Math|Rotator|MakeRotator 0.0 (* AxisValue 1.5) 0.0) false false))

(event Input|AxisEvents|InputAxisMoveForward
  (params (AxisValue :type Float%20%28single-precision%29))
  ;[1 1 1] Move input
  (Class|TankMovementComponent|IntendMoveForward (Variables|Default|GetTankMovement) AxisValue))

(event Input|AxisEvents|InputAxisTurnClockwise
  (params (AxisValue :type Float%20%28single-precision%29))
  ;[1 1 1] Move input
  (Class|TankMovementComponent|IntendRotateClockwise (Variables|Default|GetTankMovement) AxisValue))

(fn ConstructionScript
  (bind _trackright (Variables|Default|GetTrackRight))
  (bind _trackleft (Variables|Default|GetTrackLeft))
  (Components|StaticMesh|SetStaticMesh _trackleft "/Game/Meshes/Tank/tank_fbx_Track.tank_fbx_Track")
  (Class|PrimitiveComponent|SetNotifyRigidBodyCollision _trackleft true)
  (Class|PrimitiveComponent|SetPhysMaterialOverride _trackleft "/Game/Meshes/Tank/Track_PM.Track_PM")
  (Components|StaticMesh|SetStaticMesh _trackright "/Game/Meshes/Tank/tank_fbx_Track.tank_fbx_Track")
  (Class|PrimitiveComponent|SetNotifyRigidBodyCollision _trackright true)
  (Class|PrimitiveComponent|SetPhysMaterialOverride _trackright "/Game/Meshes/Tank/Track_PM.Track_PM"))

(fn InitializeHealthBarWidget
  (bind _ashealth_bar (Utilities|Casting|CastToHealthBar (UserInterface|GetUserWidgetObject (Variables|Default|GetWidget))))
  (Variables|/Game/Widgets/HealthBar.HealthBar_C|SetMyTank _ashealth_bar self))